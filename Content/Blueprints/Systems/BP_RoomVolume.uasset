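; BP_RoomVolume is a trigger volume that marks a room, tagged with RoomID, as watched when the player character enters its box.
; That overlap sets IsWatched and binds handlers to the watched and unwatched events, using GetActorOfClass on its own class for the watched binding.
; The handlers only print debug text, with Watched and Unwatched labels swapped.
; Nothing here broadcasts those events or clears IsWatched, as end overlap is empty.
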(event OnComponentBeginOverlap(Box)
  (params (OverlappedComponent :type Primitive%20Component%20Object%20Reference) (OtherActor :type Actor%20Object%20Reference) (OtherComp :type Primitive%20Component%20Object%20Reference) (OtherBodyIndex :type Integer) (bFromSweep :type Boolean) (SweepResult :type Hit%20Result%20Structure%20%28by%20ref%29))
  (if (== (Game|GetPlayerCharacter 0) OtherActor)
    (Variables|Default|SetbIsWatched true)
    (Development|PrintString (Utilities|String|ToString(Boolean) (Variables|Default|GetbIsWatched)))
    (bind _returnvalue (Actor|GetActorOfClass "BP_RoomVolume_C"))
    (for _array_element (Utilities|Array|MakeArray _returnvalue)
      (EventDispatchers|BindEventtoOnRoomWatched (delegate Custom|HandleRoomWatched)))
    (EventDispatchers|BindEventtoOnRoomUnwatched (delegate Custom|HandleRoomUnwatched))))

(event OnComponentEndOverlap(Box)
  (params (OverlappedComponent :type Primitive%20Component%20Object%20Reference) (OtherActor :type Actor%20Object%20Reference) (OtherComp :type Primitive%20Component%20Object%20Reference) (OtherBodyIndex :type Integer)))

(event Custom|HandleRoomWatched
  (Development|PrintString (Utilities|String|Append "Unwatched" (Utilities|String|ToString(Name) (Variables|Default|GetRoomID)))))

(event Custom|HandleRoomUnwatched
  (Development|PrintString (Utilities|String|Append "Watched" (Utilities|String|ToString(Name) (Variables|Default|GetRoomID)))))

(event EventBeginPlay)

(event Collision|EventActorBeginOverlap
  (params (OtherActor :type Actor%20Object%20Reference)))

(event EventTick
  (params (DeltaSeconds :type Float%20%28single-precision%29)))

(fn ConstructionScript)